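; BP_Marking is a marker actor in Disaster_VR that shows a text label on a widget component.
; On BeginPlay it casts the component's user widget to Marking_Label and passes its own LabelText into it.
; Every Tick it rotates the widget toward the player camera with a look-at rotation, so the label always faces the viewer.
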(event `self.ReceiveBeginPlay`
  (bind _asmarking_label (cast `/Game/Disaster_VR/Marking_Label` (`WidgetComponent.GetUserWidgetObject` (`self.Widget`))))
  (set `/Game/Disaster_VR/Marking_Label.Label Text` (`self.Label Text`) _asmarking_label))

(event `self.ReceiveTick`
  (params (DeltaSeconds :type "Float (single-precision)"))
  (`SceneComponent.K2_SetWorldRotation` (`self.Widget`) (`KismetMathLibrary.FindLookAtRotation` (`SceneComponent.K2_GetComponentLocation` (`self.Widget`)) (`PlayerCameraManager.GetCameraLocation` (`GameplayStatics.GetPlayerCameraManager` 0))) false false))

(fn `UserConstructionScript`)