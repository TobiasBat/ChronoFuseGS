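; Player character for viewing and evaluating a SplattingActor scene, with free-flight, auto-orbit and training-camera view modes.
; Modes reattach one camera to the spring arm or a training camera actor, copying the latter's FOV.
; Input actions switch the splat's render mode, time selection and camera indicators, and start an FPS test.
; BP_ScreenCapturer saves screenshots named by view and time selection, including delay-driven recursive batches over camera sequences and time combinations.
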(event `EnhancedInput|/Game/Input/IA_Next_Camera`
  (params (ActionValue :type Boolean) (ElapsedSeconds :type "Float (double-precision)") (TriggeredSeconds :type "Float (double-precision)") (InputAction :type "InputAction Object Reference" :default "/Game/Input/IA_Next_Camera.IA_Next_Camera"))
  ; Test Cameras
  (:`Triggered`
    (bind _returnvalue (`GameplayStatics.GetActorOfClass` "/Script/ChronoFuseGS.SplattingActor" :!label _label))
    (bind _returnvalue_2 (`SplattingActor.GetNextCameraIndex` _returnvalue (`self.Camera Index`) 1))
    (set `self.Camera Index` _returnvalue_2)
    (`self.Set Camera to Train Camera Index`)))

(event `Switch_To_Next_Camera`
  ; Test Cameras
  (goto _label))

(event `EnhancedInput|/Game/Input/IA_Prev_Camera`
  (params (ActionValue :type Boolean) (ElapsedSeconds :type "Float (double-precision)") (TriggeredSeconds :type "Float (double-precision)") (InputAction :type "InputAction Object Reference" :default "/Game/Input/IA_Prev_Camera.IA_Prev_Camera"))
  ; Test Cameras
  (:`Triggered`
    (bind _returnvalue (`GameplayStatics.GetActorOfClass` "/Script/ChronoFuseGS.SplattingActor"))
    (bind _returnvalue_2 (`SplattingActor.GetNextCameraIndex` _returnvalue (`self.Camera Index`) -1))
    (set `self.Camera Index` _returnvalue_2)
    (`self.Set Camera to Train Camera Index`)))

(event `Sert Camera Rotation and Location`
  (params (location :type "Vector Structure") (rotation :type "Rotator Structure"))
  (`SceneComponent.K2_SetWorldLocationAndRotation` (`self.Camera`) location rotation false true))

(event `EnhancedInput|/Game/Input/Render_Mode/IA_RenderMode_ChangeHighlight`
  (params (ActionValue :type Boolean) (ElapsedSeconds :type "Float (double-precision)") (TriggeredSeconds :type "Float (double-precision)") (InputAction :type "InputAction Object Reference" :default "/Game/Input/Render_Mode/IA_RenderMode_ChangeHighlight.IA_RenderMode_ChangeHighlight"))
  ; Switch Render Modes of Splatting Actor
  (:`Triggered`
    (`SplattingActor.SetRenderMode` (`self.Splatting Actor`) 4)))

(event `EnhancedInput|/Game/Input/Render_Mode/IA_RenderMode_Color`
  (params (ActionValue :type Boolean) (ElapsedSeconds :type "Float (double-precision)") (TriggeredSeconds :type "Float (double-precision)") (InputAction :type "InputAction Object Reference" :default "/Game/Input/Render_Mode/IA_RenderMode_Color.IA_RenderMode_Color"))
  ; Switch Render Modes of Splatting Actor
  (:`Triggered`
    (`SplattingActor.SetRenderMode` (`self.Splatting Actor`) 0)))

(event `EnhancedInput|/Game/Input/Render_Mode/IA_RenderMode_Change`
  (params (ActionValue :type Boolean) (ElapsedSeconds :type "Float (double-precision)") (TriggeredSeconds :type "Float (double-precision)") (InputAction :type "InputAction Object Reference" :default "/Game/Input/Render_Mode/IA_RenderMode_Change.IA_RenderMode_Change"))
  ; Switch Render Modes of Splatting Actor
  (:`Triggered`
    (`SplattingActor.SetRenderMode` (`self.Splatting Actor`) 1)))

(event `EnhancedInput|/Game/Input/Render_Mode/IA_RenderMode_Reuse`
  (params (ActionValue :type Boolean) (ElapsedSeconds :type "Float (double-precision)") (TriggeredSeconds :type "Float (double-precision)") (InputAction :type "InputAction Object Reference" :default "/Game/Input/Render_Mode/IA_RenderMode_Reuse.IA_RenderMode_Reuse"))
  ; Switch Render Modes of Splatting Actor
  (:`Triggered`
    (`SplattingActor.SetRenderMode` (`self.Splatting Actor`) 2)))

(event `EnhancedInput|/Game/Input/Render_Mode/IA_RenderMode_ColorActivation`
  (params (ActionValue :type Boolean) (ElapsedSeconds :type "Float (double-precision)") (TriggeredSeconds :type "Float (double-precision)") (InputAction :type "InputAction Object Reference" :default "/Game/Input/Render_Mode/IA_RenderMode_ColorActivation.IA_RenderMode_ColorActivation"))
  ; Switch Render Modes of Splatting Actor
  (:`Triggered`
    (`SplattingActor.SetRenderMode` (`self.Splatting Actor`) 3)))

(event `EnhancedInput|/Game/Input/Time/IA_NextTime`
  (params (ActionValue :type Boolean) (ElapsedSeconds :type "Float (double-precision)") (TriggeredSeconds :type "Float (double-precision)") (InputAction :type "InputAction Object Reference" :default "/Game/Input/Time/IA_NextTime.IA_NextTime"))
  ; Switch Render Modes of Splatting Actor
  (:`Triggered`
    (`SplattingActor.ShowNextTimeSelection` (`self.Splatting Actor`) 1)))

(event `EnhancedInput|/Game/Input/Time/IA_PrevTime`
  (params (ActionValue :type Boolean) (ElapsedSeconds :type "Float (double-precision)") (TriggeredSeconds :type "Float (double-precision)") (InputAction :type "InputAction Object Reference" :default "/Game/Input/Time/IA_PrevTime.IA_PrevTime"))
  ; Switch Render Modes of Splatting Actor
  (:`Triggered`
    (`SplattingActor.ShowNextTimeSelection` (`self.Splatting Actor`) -1)))

(event `EnhancedInput|/Game/Input/Time/IA_AllTime`
  (params (ActionValue :type Boolean) (ElapsedSeconds :type "Float (double-precision)") (TriggeredSeconds :type "Float (double-precision)") (InputAction :type "InputAction Object Reference" :default "/Game/Input/Time/IA_AllTime.IA_AllTime"))
  ; Switch Render Modes of Splatting Actor
  (:`Triggered`
    (`SplattingActor.ShowAllTimes` (`self.Splatting Actor`))))

(event `EnhancedInput|/Game/Input/IA_Turn_Right`
  (params (ActionValue :type "Float (double-precision)") (ElapsedSeconds :type "Float (double-precision)") (TriggeredSeconds :type "Float (double-precision)") (InputAction :type "InputAction Object Reference" :default "/Game/Input/IA_Turn_Right.IA_Turn_Right"))
  ; FPV Character Movement
  (:`Triggered`
    (if (`self.Move Character`)
      (`self.AddControllerYawInput` ActionValue))))

(event `EnhancedInput|/Game/Input/IA_Zoom_In`
  (params (ActionValue :type Boolean) (ElapsedSeconds :type "Float (double-precision)") (TriggeredSeconds :type "Float (double-precision)") (InputAction :type "InputAction Object Reference" :default "/Game/Input/IA_Zoom_In.IA_Zoom_In"))
  (bind _array (`|MakeArray` 3500.0 1500.0 2500.0))
  (:`Triggered`
    (bind _output_get (set `self.Arm_Lengths` _array))
    (set `SpringArmComponent.TargetArmLength` (`|GetArrayItem` _output_get (`self.Arm_Length_Index`)) (`self.SpringArm`))
    (set `self.Arm_Length_Index` (mod (+ (`self.Arm_Length_Index`) 1) (`KismetArrayLibrary.Array_Length` _array)))))

(event `EnhancedInput|/Game/Input/IA_Turn_Up`
  (params (ActionValue :type "Float (double-precision)") (ElapsedSeconds :type "Float (double-precision)") (TriggeredSeconds :type "Float (double-precision)") (InputAction :type "InputAction Object Reference" :default "/Game/Input/IA_Turn_Up.IA_Turn_Up"))
  ; FPV Character Movement
  (:`Triggered`
    (if (`self.Move Character`)
      (`self.AddControllerPitchInput` ActionValue))))

(event `EnhancedInput|/Game/Input/IA_Move_Forward`
  (params (ActionValue :type "Float (double-precision)") (ElapsedSeconds :type "Float (double-precision)") (TriggeredSeconds :type "Float (double-precision)") (InputAction :type "InputAction Object Reference" :default "/Game/Input/IA_Move_Forward.IA_Move_Forward"))
  ; FPV Character Movement
  (:`Triggered`
    (if (`self.Move Character`)
      (`self.AddMovementInput` (`SceneComponent.GetForwardVector` (`self.CapsuleComponent`)) ActionValue))))

(event `EnhancedInput|/Game/Input/IA_FPV_Camera`
  (params (ActionValue :type Boolean) (ElapsedSeconds :type "Float (double-precision)") (TriggeredSeconds :type "Float (double-precision)") (InputAction :type "InputAction Object Reference" :default "/Game/Input/IA_FPV_Camera.IA_FPV_Camera"))
  ; FPV Camera
  (:`Triggered`
    (set `self.CameraOrbitting` false)
    (set `SpringArmComponent.bUsePawnControlRotation` true (`self.SpringArm`))
    (set `SpringArmComponent.TargetArmLength` 0.0 (`self.SpringArm`))
    (`SceneComponent.K2_AttachToComponent` (`self.Camera`) (`self.SpringArm`) "None" "KeepRelative" "KeepRelative" "KeepRelative" true)
    (set `self.Move Character` true)))

(event `EnhancedInput|/Game/Input/IA_Move_Right`
  (params (ActionValue :type "Float (double-precision)") (ElapsedSeconds :type "Float (double-precision)") (TriggeredSeconds :type "Float (double-precision)") (InputAction :type "InputAction Object Reference" :default "/Game/Input/IA_Move_Right.IA_Move_Right"))
  ; FPV Character Movement
  (:`Triggered`
    (if (`self.Move Character`)
      (`self.AddMovementInput` (`SceneComponent.GetRightVector` (`self.CapsuleComponent`)) ActionValue))))

(event `Start_Stop_Orbit`
  ; Orbit Camera
  (`SceneComponent.K2_AttachToComponent` (`self.Camera`) (`self.SpringArm`) "None" "KeepRelative" "KeepRelative" "KeepRelative" true :!label _label_2)
  (set `self.Move Character` false)
  (bind _outactors (`GameplayStatics.GetAllActorsOfClass` "/Game/BP/BP_Orbit_Center.BP_Orbit_Center_C"))
  (`self.K2_SetActorLocationAndRotation` (`self.K2_GetActorLocation` (`|GetArrayItem` _outactors)) (struct) false true)
  (`Controller.SetControlRotation` (`GameplayStatics.GetPlayerController` 0) (`KismetMathLibrary.MakeRotator` 0.0 -30.0))
  (set `SpringArmComponent.TargetArmLength` 8000.0 (`self.SpringArm`))
  (set `self.CameraOrbitting` true))

(event `EnhancedInput|/Game/Input/IA_Orbit_Camera`
  (params (ActionValue :type Boolean) (ElapsedSeconds :type "Float (double-precision)") (TriggeredSeconds :type "Float (double-precision)") (InputAction :type "InputAction Object Reference" :default "/Game/Input/IA_Orbit_Camera.IA_Orbit_Camera"))
  ; Orbit Camera
  (:`Triggered`
    (set `self.orbit_center_index` 0)
    (goto _label_2)))

(event `EnhancedInput|/Game/Input/IA_Move_Up`
  (params (ActionValue :type "Float (double-precision)") (ElapsedSeconds :type "Float (double-precision)") (TriggeredSeconds :type "Float (double-precision)") (InputAction :type "InputAction Object Reference" :default "/Game/Input/IA_Move_Up.IA_Move_Up"))
  ; FPV Character Movement
  (:`Triggered`
    (if (`self.Move Character`)
      (`self.AddMovementInput` (`SceneComponent.GetUpVector` (`self.CapsuleComponent`)) ActionValue))))

(event `EnhancedInput|/Game/Input/IA_Toogle_Camera_Indicators`
  (params (ActionValue :type Boolean) (ElapsedSeconds :type "Float (double-precision)") (TriggeredSeconds :type "Float (double-precision)") (InputAction :type "InputAction Object Reference" :default "/Game/Input/IA_Toogle_Camera_Indicators.IA_Toogle_Camera_Indicators"))
  ; Toggle Camera Indicators
  (:`Triggered`
    (bind _returnvalue (`GameplayStatics.GetActorOfClass` "/Script/ChronoFuseGS.SplattingActor"))
    (bind _output_get (set `SplattingActor.ShowCameraIndicators` (not (`SplattingActor.ShowCameraIndicators` _returnvalue)) _returnvalue))
    (`SplattingActor.SetCameraIndicatorVisibility` _returnvalue _output_get)))

(event `self.ReceiveTick`
  (params (DeltaSeconds :type "Float (single-precision)"))
  (bind _returnvalue (`GameplayStatics.GetPlayerController` 0))
  ; Orbit Camera
  (if (`self.CameraOrbitting`)
    (`Controller.SetControlRotation` _returnvalue (`KismetMathLibrary.MakeRotator` (.roll (`Controller.GetControlRotation` _returnvalue)) (.pitch (`Controller.GetControlRotation` _returnvalue)) (+ (.yaw (`Controller.GetControlRotation` _returnvalue)) (* DeltaSeconds (`self.orbit_speed`)))))))

(event `EnhancedInput|/Game/Input/IA_Play_Pause`
  (params (ActionValue :type Boolean) (ElapsedSeconds :type "Float (double-precision)") (TriggeredSeconds :type "Float (double-precision)") (InputAction :type "InputAction Object Reference" :default "/Game/Input/IA_Play_Pause.IA_Play_Pause"))
  ; Orbit Camera
  (:`Triggered`
    (if (> (`self.orbit_speed`) 0.01)
      (set `self.orbit_speed` 0.0)
      (set `self.CameraOrbitting` false)
      (else
        (set `self.orbit_speed` 10.0)
        (set `self.CameraOrbitting` true)))))

(event `self.ReceiveBeginPlay`
  ; Loading Input subsystem
  (bind _asplayer_controller (cast `PlayerController` (`self.GetController`)))
  (`EnhancedInputSubsystemInterface.AddMappingContext` (pcsubsystem `EnhancedInputLocalPlayerSubsystem` _asplayer_controller) "/Game/Input/IMC_Flying.IMC_Flying" 0 (struct))
  (bind _returnvalue (`GameplayStatics.GetActorOfClass` "/Script/ChronoFuseGS.SplattingActor"))
  (set `self.Splatting Actor` _returnvalue)
  (bind _returnvalue_2 (`GameplayStatics.GetActorOfClass` "/Game/ScreenCapturer/BP_ScreenCapturer.BP_ScreenCapturer_C"))
  (set `self.ScreenCapturer` _returnvalue_2)
  (set `self.orbit_speed` 10.0))

(event `Pause Camera  Orbit`
  ; Orbit Camera
  (set `self.CameraOrbitting` false))

(event `EnhancedInput|/Game/Input/IA_Make_Screenshot`
  (params (ActionValue :type Boolean) (ElapsedSeconds :type "Float (double-precision)") (TriggeredSeconds :type "Float (double-precision)") (InputAction :type "InputAction Object Reference" :default "/Game/Input/IA_Make_Screenshot.IA_Make_Screenshot"))
  ; Take Screenshots
  (:`Triggered`
    (`self.Make Screenshot`)))

(event `Make Screenshot`
  ; Take Screenshots
  (`self.Update Capture File Name`)
  (`ScreenCapturer.TakeScreenshot` (`self.ScreenCapturer`) (`self.Screenshot File Name`)))

(event `EnhancedInput|/Game/Input/IA_Capture_Sequence`
  (params (ActionValue :type Boolean) (ElapsedSeconds :type "Float (double-precision)") (TriggeredSeconds :type "Float (double-precision)") (InputAction :type "InputAction Object Reference" :default "/Game/Input/IA_Capture_Sequence.IA_Capture_Sequence"))
  ; Take Screenshots
  (:`Triggered`
    (`KismetSystemLibrary.PrintText` "Capturing Sequence")
    (set `self.capture_sequence_index` 0)
    (`self.Capture Sequence Curr Index`)))

(event `Capture Sequence Curr Index`
  ; Take Screenshots
  (bind _returnvalue (`GameplayStatics.GetActorOfClass` "/Game/ScreenCapturer/BP_ScreenCapturer.BP_ScreenCapturer_C"))
  (bind _capturesequencecamerasindex (`ScreenCapturer.CaptureSequenceCamerasIndex` _returnvalue))
  (set `self.Camera Index` (`|GetArrayItem` _capturesequencecamerasindex (`self.capture_sequence_index`)))
  (`self.Set Camera to Train Camera Index`)
  (`KismetSystemLibrary.Delay` 0.2)
  (`self.Make Screenshot`)
  (bind _output_get (set `self.capture_sequence_index` (+ (`self.capture_sequence_index`) 1)))
  (if (< _output_get (`KismetArrayLibrary.Array_Length` _capturesequencecamerasindex))
    (`KismetSystemLibrary.Delay` 1.0)
    (`self.Capture Sequence Curr Index`)
    (else
      (`KismetSystemLibrary.PrintText` "Capturing Sequence Done"))))

(event `EnhancedInput|/Game/Input/IA_AllTimeCombinationScreenshot`
  (params (ActionValue :type Boolean) (ElapsedSeconds :type "Float (double-precision)") (TriggeredSeconds :type "Float (double-precision)") (InputAction :type "InputAction Object Reference" :default "/Game/Input/IA_AllTimeCombinationScreenshot.IA_AllTimeCombinationScreenshot"))
  ; Take Screenshots
  (:`Triggered`
    (bind _returnvalue (`GameplayStatics.GetActorOfClass` "/Game/gsp/BP_SplattingActor.BP_SplattingActor_C"))
    (set `self.capture_sequence_index` 1)
    (`self.Capture Time Combination`)))

(event `Capture Time Combination`
  ; Take Screenshots
  (bind _returnvalue (`ScreenCapturer.GetTimeCombination` (`self.ScreenCapturer`) (`self.capture_sequence_index`)))
  (`SplattingActor.SetTimeSelection` (stale `EnhancedInput|/Game/Input/IA_AllTimeCombinationScreenshot` _returnvalue) _returnvalue)
  (`KismetSystemLibrary.Delay` 1.0)
  (`self.Make Screenshot`)
  (bind _output_get (set `self.capture_sequence_index` (+ (`self.capture_sequence_index`) 1)))
  (bind _returnvalue_2 (`SplattingActor.NumberOfTimes` (stale `EnhancedInput|/Game/Input/IA_AllTimeCombinationScreenshot` _returnvalue)))
  (if (< _output_get (* _returnvalue_2 _returnvalue_2))
    (`self.Capture Time Combination`)))

(event `EnhancedInput|/Game/Input/IA_Start_FPS_Test`
  (params (ActionValue :type Boolean) (ElapsedSeconds :type "Float (double-precision)") (TriggeredSeconds :type "Float (double-precision)") (InputAction :type "InputAction Object Reference" :default "/Game/Input/IA_Start_FPS_Test.IA_Start_FPS_Test"))
  (:`Triggered`
    (`KismetSystemLibrary.PrintString` "Starting FPS Test")
    (bind _returnvalue (`GameplayStatics.GetActorOfClass` "/Game/gsp/BP_SplattingActor.BP_SplattingActor_C"))
    (`SplattingActor.StartFPSTest` _returnvalue 25)))

(fn `Set Camera to Train Camera Index`
  (bind _camera_index (`self.Camera Index`))
  (set `self.CameraOrbitting` false)
  (set `self.Move Character` false)
  (bind _returnvalue (`GameplayStatics.GetActorOfClass` "/Script/ChronoFuseGS.SplattingActor"))
  (bind _returnvalue_2 (`SplattingActor.GetCameraActor` _returnvalue (`self.Camera Index`)))
  (`SceneComponent.K2_AttachToComponent` (`self.Camera`) (`Actor.RootComponent` _returnvalue_2) "None" "KeepRelative" "KeepRelative" "KeepRelative" true)
  (bind _returnvalue_3 (`SplattingActor.GetFieldOfView` _returnvalue _camera_index))
  (`CameraComponent.SetFieldOfView` (`self.Camera`) _returnvalue_3)
  (`KismetSystemLibrary.PrintText` (`KismetTextLibrary.Conv_StringToText` (`KismetStringLibrary.BuildString_Int` "" "Selected Camera Index" _camera_index))))

(fn `Update Capture File Name`
  (bind (_year _month _day _hour _minute _second) (`KismetMathLibrary.BreakDateTime` (`KismetMathLibrary.Now`)))
  (bind _result (`|FormatText` "{Year}-{Month}-{Day}-{Hour}-{Minute}-{Sec}" _year _month _day _hour _minute _second))
  (bind _returnvalue (`GameplayStatics.GetActorOfClass` "/Script/ChronoFuseGS.SplattingActor"))
  (bind _returnvalue_2 (`SplattingActor.GetCameraNameFromIndex` _returnvalue (`self.Camera Index`)))
  (bind _returnvalue_3 (`SplattingActor.GetTimeSelectionRepresentation` _returnvalue))
  (if (and (not (`self.CameraOrbitting`)) (not (`self.Move Character`)))
    (set `self.Screenshot File Name` (`KismetTextLibrary.Conv_TextToString` (`|FormatText` "Camera_{CName}_I{index}_ActS-{act_selection}_T-{time}.png" _returnvalue_2 (`self.Camera Index`) _returnvalue_3 _result)))
    (elif (`self.CameraOrbitting`)
      (set `self.Screenshot File Name` (`KismetTextLibrary.Conv_TextToString` (`|FormatText` "Orbit_{arm_length}_ActS-{act_selection}_T-{time}.png" (`SpringArmComponent.TargetArmLength` (`self.SpringArm`)) _returnvalue_3 _result)))
      (else
        (set `self.Screenshot File Name` (`KismetTextLibrary.Conv_TextToString` (`|FormatText` "FPV__ActS-{act_selection}_T-{time}.png" _returnvalue_3 _result)))))))

(fn `UserConstructionScript`)